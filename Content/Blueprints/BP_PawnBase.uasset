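; BP_PawnBase is a player pawn that shifts sideways between discrete lanes on Left and Right input.
; On BeginPlay it reads lane count and width from the level manager and sets its current lane to the middle.
; Each press, ignored while moving or at an edge lane, plays a timeline that lerps Y from the live location toward the neighboring lane.
; The lane index updates when the timeline finishes.
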(event `self.ReceiveBeginPlay`
  (`self.Initialise`))

(event `InputAction|Left`
  (params (Key :type "Key Structure"))
  (bind (_returnvalue_x _returnvalue_y) (`KismetMathLibrary.BreakVector` (`self.K2_GetActorLocation`)))
  (bind (_returnvalue_x_2 _returnvalue_y_2 _returnvalue_z) (`KismetMathLibrary.BreakVector` (`self.K2_GetActorLocation`)))
  ;[0 0.6529 1] Izquierda pre
  (:`Pressed`
    (if (<= (`self.CurrentLane`) 1)
      _
      (elif (not (`self.bMoving`))
        (set `self.bMoving` true)
        (set `self.TargetPosition` (- _returnvalue_y (`self.LaneWidth`)))
        (bind (_direction _newtrack_0) (`Timeline|MoveLeft`)
          (:`Update`
            (`self.K2_SetActorLocation` (`KismetMathLibrary.MakeVector` _returnvalue_x_2 (`KismetMathLibrary.Lerp` _returnvalue_y_2 (`self.TargetPosition`) _newtrack_0) _returnvalue_z)))
          (:`Finished`
            (set `self.bMoving` false)
            (`/Engine/EditorBlueprintResources/StandardMacros.DecrementInt` (`self.CurrentLane`))))))))

(event `InputAction|Right`
  (params (Key :type "Key Structure"))
  (bind (_returnvalue_x _returnvalue_y) (`KismetMathLibrary.BreakVector` (`self.K2_GetActorLocation`)))
  (bind (_returnvalue_x_2 _returnvalue_y_2 _returnvalue_z) (`KismetMathLibrary.BreakVector` (`self.K2_GetActorLocation`)))
  ;[0 1 0.5191] Comment
  (:`Pressed`
    ;;[1 1 1] Comprueba si fue presionado Derecha cuando esta en la linea derecha
    (if (== (`self.CurrentLane`) (`/Game/Blueprints/BP_LevelManager.NumberOfLanes` (`self.LevelManagerRef`)))
      _
      (elif (not (`self.bMoving`))
        (set `self.bMoving` true)
        (set `self.TargetPosition` (+ _returnvalue_y (`self.LaneWidth`)))
        (bind (_direction _newtrack_0) (`Timeline|MoveRight`)
          (:`Update`
            (`self.K2_SetActorLocation` (`KismetMathLibrary.MakeVector` _returnvalue_x_2 (`KismetMathLibrary.Lerp` _returnvalue_y_2 (`self.TargetPosition`) _newtrack_0) _returnvalue_z)))
          (:`Finished`
            (set `self.bMoving` false)
            (`/Engine/EditorBlueprintResources/StandardMacros.IncrementInt` (`self.CurrentLane`))))))))

(fn `Initialise`
  (bind _output (`/Game/Blueprints/BPM_Lib.GetLevelManager`)
    (:`Is Valid`
      (set `self.LevelManagerRef` _output)
      (set `self.CurrentLane` (+ (/ (`/Game/Blueprints/BP_LevelManager.NumberOfLanes` (`self.LevelManagerRef`)) 2) 1))
      (set `self.LaneWidth` (`/Game/Blueprints/BP_LevelManager.LaneWidth` (`self.LevelManagerRef`))))
    (:`Is Not Valid`
      (`KismetSystemLibrary.PrintString` "no_level_manager_found" true true (struct :`R` 0.81 :`A` 1.0)))))

(fn `UserConstructionScript`)