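; BP_ScrollingComponent is an actor component that scrolls its owning actor at the level's shared speed.
; On BeginPlay it looks up the level manager and caches the reference if found.
; Each Tick it scales the owner's forward vector by LevelSpeed and delta time, then applies it as a local-space offset without sweep, reading the manager without a validity check.
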(event `self.ReceiveBeginPlay`
  (bind (_levelmanagerfound _levelmanager) (`/Game/Blueprints/Libs/BPF_Lib.GetLevelManager`))
  (if _levelmanagerfound
    (set `self.LevelManagerRef` _levelmanager)))

(event `self.ReceiveTick`
  (params (DeltaSeconds :type "Float (single-precision)"))
  (set `self.deltaSeconds` DeltaSeconds)
  (bind _output_get (set `self.Movement` (* (* (`Actor.GetActorForwardVector` (`self.GetOwner`)) (`/Game/Blueprints/BP_LevelManager.LevelSpeed` (`self.LevelManagerRef`))) (`self.deltaSeconds`))))
  (`Actor.K2_AddActorLocalOffset` (`self.GetOwner`) _output_get false false))